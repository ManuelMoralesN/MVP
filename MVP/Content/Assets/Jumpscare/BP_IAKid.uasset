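; BP_IAKid is an enemy AI character that wanders, chases the player on sight and plays a jumpscare attack.
; After a startup delay it loops between random reachable points, with footsteps (Pasos) active only while moving on the ground.
; PawnSensing triggers the chase, and a retriggerable delay returns it to wandering after sightings stop or an attack completes.
; Reaching the player plays the montage, whose notify runs a sphere trace to apply damage.
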(event `self.ReceiveBeginPlay`
  (`KismetSystemLibrary.Delay` 30.0)
  (`self.GoToRandomPoint`))

(event `self.ReceiveTick`
  (params (DeltaSeconds :type "Float (single-precision)"))
  (bind _pasos (`self.Pasos`))
  (if (> (`KismetMathLibrary.VSize` (`MovementComponent.Velocity` (`self.CharacterMovement`))) 0.0)
    (if (`NavMovementInterface.IsFalling` (`self.CharacterMovement`))
      (`ActorComponent.Deactivate` _pasos :!label _label)
      (else
        (`ActorComponent.Activate` _pasos false)))
    (else
      (goto _label))))

(event `GoToRandomPoint`
  ;[0.15 0.03639 0.1191 0.5] IA puntos aleatorios
  (`|AIMoveTo` self (`NavigationSystemV1.K2_GetRandomReachablePointInRadius` (`self.K2_GetActorLocation`) 2500.0 null null) null
    (:`OnSuccess`
      (`KismetSystemLibrary.Delay` 5.0)
      (`self.GoToRandomPoint`))))

(event `self.PawnSensing.OnSeePawn`
  (params (Pawn :type "Pawn Object Reference"))
  ;[0.1494 0.15 0.03453 0.5] Seguir y perder
  (`|ExecutionSequence`
    (:`then_0`
      (if (not (`self.bIsAtacking`))
        (`|AIMoveTo` self (0.0 0.0 0.0) (`GameplayStatics.GetPlayerPawn` 0)
          (:`OnSuccess`
            (`self.Attack`)))))
    (:`then_1`
      (`KismetSystemLibrary.RetriggerableDelay` 2.0 :!label _label_2)
      (if (not (`self.bIsAtacking`))
        (`self.GoToRandomPoint`)))))

(event `Attack`
  (bind _attackpointtrace (`self.AttackPointTrace`))
  (bind _returnvalue (`SceneComponent.K2_GetComponentLocation` _attackpointtrace))
  (if (not (`self.bIsAtacking`))
    (set `self.bIsAtacking` true)
    (`|PlayMontage` (`self.Mesh`) "/Game/Assets/Jumpscare/AnimationsJumps/SUP_GUYS_ITS_YOUR_GIRL_AGATHA_AND_WELCOME_TO_DARK_DECEPTION_Anim_agatha_RIG_skeleton_jumpscare2_Montage.SUP_GUYS_ITS_YOUR_GIRL_AGATHA_AND_WELCOME_TO_DARK_DECEPTION_Anim_agatha_RIG_skeleton_jumpscare2_Montage"
      (:`OnCompleted`
        (set `self.bIsAtacking` false)
        (goto _label_2))
      (:`OnNotifyBegin`
        ;[0 0.15 0.1339 0.5] Detect Damage
        (bind (_outhit _returnvalue_2) (`KismetSystemLibrary.SphereTraceSingleForObjects` _returnvalue (+ _returnvalue (* (`SceneComponent.GetForwardVector` _attackpointtrace) 50.0)) 20.0 (`|MakeArray` "ObjectTypeQuery3" :!type "EObjectTypeQuery Enum")))
        (if _returnvalue_2
          (`GameplayStatics.ApplyDamage` (`.HitActor` (`GameplayStatics.BreakHitResult` _outhit)) 5.0))))))

(fn `UserConstructionScript`)