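; Jumpscare trigger actor that flings a set of books when the player walks into it.
; A Box overlap fires once through a DoOnce, then checks for the player character before playing a 2D scream sound and enabling physics on the book meshes with a strong one-axis force.
; Because the DoOnce sits before the player check, any earlier overlapping actor uses up the scare.
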(event `self.Box.OnComponentBeginOverlap`
  (params (OverlappedComponent :type "PrimitiveComponent Object Reference") (OtherActor :type "Actor Object Reference") (OtherComp :type "PrimitiveComponent Object Reference") (OtherBodyIndex :type Integer) (bFromSweep :type Boolean) (SweepResult :type "HitResult Structure (by ref)"))
  (bind _books (`self.Books`))
  (`/Engine/EditorBlueprintResources/StandardMacros.DoOnce` false
    (:`Completed`
      (if (== OtherActor (`GameplayStatics.GetPlayerCharacter` 0))
        (`GameplayStatics.PlaySound2D` "/Game/Assets/Sonidos/scream-with-echo-46585.scream-with-echo-46585" 0.2 1.0 0.0 null null)
        (`PrimitiveComponent.SetSimulatePhysics` _books true)
        (`PrimitiveComponent.SetSimulatePhysics` (`self.Books7`) true)
        (`PrimitiveComponent.SetSimulatePhysics` (`self.Books8`) true)
        (`PrimitiveComponent.SetSimulatePhysics` (`self.Books9`) true)
        (`PrimitiveComponent.SetSimulatePhysics` (`self.Books10`) true)
        (`PrimitiveComponent.SetSimulatePhysics` (`self.Books6`) true)
        (`PrimitiveComponent.SetSimulatePhysics` (`self.Books1`) true)
        (`PrimitiveComponent.SetSimulatePhysics` (`self.Books2`) true)
        (`PrimitiveComponent.SetSimulatePhysics` (`self.Books11`) true)
        (`PrimitiveComponent.SetSimulatePhysics` (`self.Books16`) true)
        (`PrimitiveComponent.SetSimulatePhysics` (`self.Books14`) true)
        (`PrimitiveComponent.SetSimulatePhysics` (`self.Books4`) true)
        (`PrimitiveComponent.AddForce` _books (-120000.0 0.0 0.0) "None" false)
        (`PrimitiveComponent.AddForce` (`self.Books7`) (-120000.0 0.0 0.0) "None" false)
        (`PrimitiveComponent.AddForce` (`self.Books8`) (-120000.0 0.0 0.0) "None" false)
        (`PrimitiveComponent.AddForce` (`self.Books9`) (-120000.0 0.0 0.0) "None" false)
        (`PrimitiveComponent.AddForce` (`self.Books10`) (-120000.0 0.0 0.0) "None" false)
        (`PrimitiveComponent.AddForce` (`self.Books6`) (-120000.0 0.0 0.0) "None" false)
        (`PrimitiveComponent.AddForce` (`self.Books1`) (-120000.0 0.0 0.0) "None" false)
        (`PrimitiveComponent.AddForce` (`self.Books2`) (-120000.0 0.0 0.0) "None" false)
        (`PrimitiveComponent.AddForce` (`self.Books11`) (-120000.0 0.0 0.0) "None" false)
        (`PrimitiveComponent.AddForce` (`self.Books16`) (-120000.0 0.0 0.0) "None" false)
        (`PrimitiveComponent.AddForce` (`self.Books14`) (-120000.0 0.0 0.0) "None" false)
        (`PrimitiveComponent.AddForce` (`self.Books4`) (-120000.0 0.0 0.0) "None" false)))))

(fn `UserConstructionScript`)