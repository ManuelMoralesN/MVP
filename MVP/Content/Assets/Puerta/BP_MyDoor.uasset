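; BP_MyDoor is a double door that opens for a player holding the required card count and leads to the win screen.
; Its DoorDetection overlap sets the character's BisinDoor flag, clears it on exit, and calls OpenDoor when Cartas equals one.
; OpenDoor plays a timeline that swings both meshes in opposite yaw directions.
; The timeline's Update pin, rather than Finished, also feeds a delay that then adds the UW_Win widget.
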(event `self.ReceiveBeginPlay`)

(event `OpenDoor`
  ;[0.15 0.07016 0.07016 0.5] Animacion de la puerta
  (bind (_direction _doorangle) (`Timeline|OpenDoorTimeline`)
    (:`Update`
      (`SceneComponent.K2_SetRelativeRotation` (`self.SM_DoubleDoor`) (`KismetMathLibrary.MakeRotator` 0.0 0.0 (* _doorangle -1.0)) false false)
      (`SceneComponent.K2_SetRelativeRotation` (`self.SM_DoubleDoor1`) (`KismetMathLibrary.MakeRotator` 0.0 0.0 _doorangle) false false)
      (`KismetSystemLibrary.Delay` 5.0)
      (bind _returnvalue (`|CreateWidget` "/Game/Assets/Widgets/UW_Win.UW_Win_C"))
      (`UserWidget.AddToViewport` _returnvalue 0))))

(event `self.DoorDetection.OnComponentBeginOverlap`
  (params (OverlappedComponent :type "PrimitiveComponent Object Reference") (OtherActor :type "Actor Object Reference") (OtherComp :type "PrimitiveComponent Object Reference") (OtherBodyIndex :type Integer) (bFromSweep :type Boolean) (SweepResult :type "HitResult Structure (by ref)"))
  ;[0 0.15 0.005471 0.5] Abrir puerta si tenemos todas las cartas
  (bind _asbp_first_person_character (cast `/Game/FirstPerson/Blueprints/BP_FirstPersonCharacter` OtherActor))
  (set `/Game/FirstPerson/Blueprints/BP_FirstPersonCharacter.bisinDoor` true _asbp_first_person_character)
  (if (== (`/Game/FirstPerson/Blueprints/BP_FirstPersonCharacter.Cartas` _asbp_first_person_character) 1)
    (`self.OpenDoor`)))

(event `self.DoorDetection.OnComponentEndOverlap`
  (params (OverlappedComponent :type "PrimitiveComponent Object Reference") (OtherActor :type "Actor Object Reference") (OtherComp :type "PrimitiveComponent Object Reference") (OtherBodyIndex :type Integer))
  ;[0 0.15 0.005471 0.5] Abrir puerta si tenemos todas las cartas
  (bind _asbp_first_person_character (cast `/Game/FirstPerson/Blueprints/BP_FirstPersonCharacter` OtherActor))
  (set `/Game/FirstPerson/Blueprints/BP_FirstPersonCharacter.bisinDoor` false _asbp_first_person_character))

(fn `UserConstructionScript`)