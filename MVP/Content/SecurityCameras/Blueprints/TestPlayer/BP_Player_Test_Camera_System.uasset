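; Test player pawn for the security camera system that walks with WASD, looks with the mouse and opens computer screens.
; Each movement key runs a short Delay loop that feeds AddMovementInput along the capsule's forward or right vector until released.
; Pressing E line-traces from the camera for an actor tagged Computer, then shows that BP_Computer's screen widget with UI-only input and a visible cursor.
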(event `InputAxisKey|MouseX`
  (params (AxisValue :type "Float (single-precision)"))
  ;[1 0.03043 0.5933 0.5913] Looking
  (`self.AddControllerYawInput` AxisValue))

(event `Key|W`
  (params (Key :type "Key Structure"))
  ;[1 0.7012 0 0.2696] Movement
  (:`Pressed`
    (set `self.W pressed` true)
    (`self.AddMovementInput` (`SceneComponent.GetForwardVector` (`self.CapsuleComponent`)) (`self.Speed`) :!label _label)
    (`KismetSystemLibrary.Delay` 1e-05)
    (if (`self.W pressed`)
      (goto _label)))
  (:`Released`
    (set `self.W pressed` false)))

(event `InputAxisKey|MouseY`
  (params (AxisValue :type "Float (single-precision)"))
  ;[1 0.03043 0.5933 0.5913] Looking
  (`self.AddControllerPitchInput` (- AxisValue (* AxisValue 2.0))))

(event `Key|S`
  (params (Key :type "Key Structure"))
  (bind _speed (`self.Speed`))
  ;[1 0.7012 0 0.2696] Movement
  (:`Pressed`
    (set `self.S pressed` true)
    (`self.AddMovementInput` (`SceneComponent.GetForwardVector` (`self.CapsuleComponent`)) (- _speed (* _speed 2.0)) :!label _label_2)
    (`KismetSystemLibrary.Delay` 1e-05)
    (if (`self.S pressed`)
      (goto _label_2)))
  (:`Released`
    (set `self.S pressed` false)))

(event `Key|E`
  (params (Key :type "Key Structure"))
  (bind _camera (`self.Camera`))
  (bind _returnvalue (`SceneComponent.K2_GetComponentLocation` _camera))
  ;[0.04794 1 0 0.5913] Enlarging the camera screen
  (:`Pressed`
    (bind (_outhit _returnvalue_2) (`KismetSystemLibrary.LineTraceSingle` _returnvalue (+ _returnvalue (* (`SceneComponent.GetForwardVector` _camera) 300.0)) "TraceTypeQuery1"))
    (if _returnvalue_2
      (bind (_bblockinghit _binitialoverlap _time _distance _location _impactpoint _normal _impactnormal _physmat _hitactor) (`GameplayStatics.BreakHitResult` _outhit))
      (if (`self.ActorHasTag` _hitactor "Computer")
        (bind _asbp_computer (cast `/Game/SecurityCameras/Blueprints/Computer/BP_Computer` _hitactor))
        (bind _returnvalue_3 (`|CreateWidget` (`GameplayStatics.GetObjectClass` (`/Game/SecurityCameras/Blueprints/Computer/BP_Computer.Belonging screen widget` _asbp_computer))))
        (`UserWidget.AddToViewport` _returnvalue_3 0)
        (`WidgetBlueprintLibrary.SetInputMode_UIOnlyEx` (`GameplayStatics.GetPlayerController` 0) null)
        (set `PlayerController.bShowMouseCursor` true (`GameplayStatics.GetPlayerController` 0))))))

(event `Key|D`
  (params (Key :type "Key Structure"))
  ;[1 0.7012 0 0.2696] Movement
  (:`Pressed`
    (set `self.D pressed` true)
    (`self.AddMovementInput` (`SceneComponent.GetRightVector` (`self.CapsuleComponent`)) (`self.Speed`) :!label _label_3)
    (`KismetSystemLibrary.Delay` 1e-05)
    (if (`self.D pressed`)
      (goto _label_3)))
  (:`Released`
    (set `self.D pressed` false)))

(event `Key|A`
  (params (Key :type "Key Structure"))
  (bind _speed (`self.Speed`))
  ;[1 0.7012 0 0.2696] Movement
  (:`Pressed`
    (set `self.A pressed` true)
    (`self.AddMovementInput` (`SceneComponent.GetRightVector` (`self.CapsuleComponent`)) (- _speed (* _speed 2.0)) :!label _label_4)
    (`KismetSystemLibrary.Delay` 1e-05)
    (if (`self.A pressed`)
      (goto _label_4)))
  (:`Released`
    (set `self.A pressed` false)))

(fn `UserConstructionScript`)